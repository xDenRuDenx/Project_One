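; BP_3 is an exercise actor that, on sphere overlap, finds numbers whose digits sum to 15 and prints them on screen.
; The overlap loop turns a counter into a string, adds its first four characters as integers, then stops past 9999 and resets the counter to 1000.
; Every Tick yaws the actor by a fixed step and reapplies a blue color to its text render.
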(event `self.Sphere.OnComponentBeginOverlap`
  (params (OverlappedComponent :type "PrimitiveComponent Object Reference") (OtherActor :type "Actor Object Reference") (OtherComp :type "PrimitiveComponent Object Reference") (OtherBodyIndex :type Integer) (bFromSweep :type Boolean) (SweepResult :type "HitResult Structure (by ref)"))
  ;[1 1 1] Exercise 3
  (for _ (range 10001)
    (bind _output_get (set `self.Var_Two` (`KismetStringLibrary.Conv_IntToString` (`self.Var_One`))))
    (bind _returnvalue (`KismetStringLibrary.GetCharacterArrayFromString` _output_get))
    (bind _output_get_2 (set `self.NewVar_0` (`KismetStringLibrary.Conv_StringToInt` (`|GetArrayItem` _returnvalue))))
    (bind _output_get_3 (set `self.NewVar_1` (`KismetStringLibrary.Conv_StringToInt` (`|GetArrayItem` _returnvalue 1))))
    (bind _output_get_4 (set `self.NewVar_2` (`KismetStringLibrary.Conv_StringToInt` (`|GetArrayItem` _returnvalue 2))))
    (bind _output_get_5 (set `self.NewVar_3` (`KismetStringLibrary.Conv_StringToInt` (`|GetArrayItem` _returnvalue 3))))
    (if (== (+ _output_get_2 _output_get_3 _output_get_4 _output_get_5) 15)
      (`KismetSystemLibrary.PrintString` (`KismetStringLibrary.Conv_IntToString` (`self.Var_One`)) true true (struct :`G` 0.66 :`B` 1.0 :`A` 1.0) 10.0))
    (bind _result (`/Engine/EditorBlueprintResources/StandardMacros.IncrementInt` (`self.Var_One`))
      (:`  `
        (if (> _result 9999)
          (break)))))
  (set `self.Var_One` 1000))

(event `self.ReceiveTick`
  (params (DeltaSeconds :type "Float (single-precision)"))
  (`self.K2_AddActorWorldRotation` (struct :`Yaw` 1.0))
  (`TextRenderComponent.SetTextRenderColor` (`self.TextRender`) (make `Color` 150)))

(fn `UserConstructionScript`)