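; Practice actor for numbered array exercises, with a spinning body and a blue-tinted TextRender updated every tick.
; Overlapping its Sphere runs a nested-loop bubble sort on ArrTest into descending order through a temporary variable, then prints each element.
; Disconnected leftovers fill VarOne with random integers, sum its negatives and multiply its non-zero odd-index values; none of these run, and BeginPlay is empty.
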(event `self.ReceiveBeginPlay`
  ;[1 1 1] Exercise 4
)

(event `self.Sphere.OnComponentBeginOverlap`
  (params (OverlappedComponent :type "PrimitiveComponent Object Reference") (OtherActor :type "Actor Object Reference") (OtherComp :type "PrimitiveComponent Object Reference") (OtherBodyIndex :type Integer) (bFromSweep :type Boolean) (SweepResult :type "HitResult Structure (by ref)"))
  (bind _arrtest (`self.ArrTest`))
  ;[0.4948 0.1328 0.0884] Exercise 7
  (for _ (`self.ArrTest`)
    (for (_array_element _array_index) (`self.ArrTest`)
      (bind _returnvalue (+ _array_index 1))
      (bind _output (`|GetArrayItem` _arrtest _returnvalue))
      (if (< (`|GetArrayItem` _arrtest _array_index) _output)
        (bind _output_get (set `self.Var_Four` _array_element))
        (`KismetArrayLibrary.Array_Set` (`self.ArrTest`) _array_index _output)
        (`KismetArrayLibrary.Array_Set` (`self.ArrTest`) _returnvalue _output_get))))
  (for _array_element_2 (`self.ArrTest`)
    (`KismetSystemLibrary.PrintString` (`KismetStringLibrary.Conv_IntToString` _array_element_2) true true (struct :`G` 0.66 :`B` 1.0 :`A` 1.0) 10.0)))

(event `self.ReceiveTick`
  (params (DeltaSeconds :type "Float (single-precision)"))
  (`self.K2_AddActorWorldRotation` (struct :`Yaw` 1.0))
  (`TextRenderComponent.SetTextRenderColor` (`self.TextRender`) (make `Color` 150)))

(fn `UserConstructionScript`)