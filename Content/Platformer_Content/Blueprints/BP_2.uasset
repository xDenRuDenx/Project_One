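; BP_2 is an exercise actor that prints a filtered number sequence when its sphere is overlapped.
; A capped loop increments VarOne, prints values whose remainder modulo 7 is 1, 2 or 5, and breaks past an upper limit.
; VarOne then resets to 35 for the next overlap.
; Tick spins the actor by a fixed, frame-rate-dependent step and reapplies a green color to its TextRender every frame.
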(event `self.Sphere.OnComponentBeginOverlap`
  (params (OverlappedComponent :type "PrimitiveComponent Object Reference") (OtherActor :type "Actor Object Reference") (OtherComp :type "PrimitiveComponent Object Reference") (OtherBodyIndex :type Integer) (bFromSweep :type Boolean) (SweepResult :type "HitResult Structure (by ref)"))
  (bind _var_one (`self.Var_One`))
  (bind _returnvalue (mod _var_one 7))
  ;[1 1 1] Exercise 2
  (for _ (range 101)
    (if (or (== _returnvalue 1) (== _returnvalue 2) (== _returnvalue 5))
      (`KismetSystemLibrary.PrintString` (`KismetStringLibrary.Conv_IntToString` _var_one) true true (struct :`G` 0.66 :`B` 1.0 :`A` 1.0) 5.0))
    (bind _result (`/Engine/EditorBlueprintResources/StandardMacros.IncrementInt` (`self.Var_One`))
      (:`  `
        (if (> _result 87)
          (break)))))
  (set `self.Var_One` 35))

(event `self.ReceiveTick`
  (params (DeltaSeconds :type "Float (single-precision)"))
  (`self.K2_AddActorWorldRotation` (struct :`Yaw` 1.0))
  (`TextRenderComponent.SetTextRenderColor` (`self.TextRender`) (make `Color` 0 100)))

(fn `UserConstructionScript`)